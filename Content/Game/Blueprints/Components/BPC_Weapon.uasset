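; BPC_Weapon is a component that spawns the player's weapon at BeginPlay and attaches it to the player mesh.
; WeaponSpawn searches weapon actors already in the level for a matching type, then spawns a new instance of that class at the data-defined socket.
; WeaponData resolves each actor's type and socket from its GunData DataTable row handle.
; The Ampersand key destroys the current weapon and spawns another type after a delay.
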(event Custom|SpawnWeapon
  (CallFunction|WeaponSpawn "/Game/Game/Blueprints/Actors/WeaponRack/BP_Weapon.BP_Weapon_C" "NewEnumerator2" (Variables|Default|GetPlayerMesh)) ; Can be replaced in event begin play ?
)

(event EventBeginPlay
  (bind _playerpawn (Class|BPIThirdPersonCharacter|GetPlayer(Message) (Components|GetOwner)))
  (Variables|Default|SetPlayerMesh (Variables|/Script/Engine.Character|GetMesh _playerpawn))
  (CallFunction|SpawnWeapon))

(event EventTick
  (params (DeltaSeconds :type Float%20%28single-precision%29)))

(event Input|KeyboardEvents|Ampersand
  (params (Key :type Key%20Structure :default "None"))
  (:Pressed
    (Actor|DestroyActor (Variables|Default|GetWeapon))
    (Utilities|FlowControl|Delay 2.0)
    (CallFunction|WeaponSpawn "/Game/Game/Blueprints/Actors/WeaponRack/BP_Weapon.BP_Weapon_C" "NewEnumerator8" (Variables|Default|GetPlayerMesh))))

(fn WeaponSpawn
  (params (Weapon :type BP%20Weapon%20Class%20Reference) (Type :type WeaponType%20Enum :default "NewEnumerator0") (PlayerMesh :type Scene%20Component%20Object%20Reference))
  (bind _outactors (Actor|GetAllActorsOfClass Weapon))
  (bind _array_element (Utilities|Array|ForEachLoopwithBreak _outactors :!label _label)
    (:LoopBody
      (bind _out_row (Utilities|WeaponData _array_element))
      (if (Utilities|Enum|Equal(Enum) (Utilities|Struct|BreakWeaponProperties _out_row) Type)
        (LocalVariables|SetLFound? (Utilities|Enum|Equal(Enum) (Utilities|Struct|BreakWeaponProperties _out_row) Type))
        (goto _label Break)))
    (:Completed
      (if (LocalVariables|GetLFound?)
        (bind _returnvalue (Game|SpawnActorfromClass (Utilities|GetClass _array_element) (Transformation|GetWorldTransform PlayerMesh) "AlwaysSpawn" 0 0))
        (bind _output_get (Variables|Default|SetWeapon _returnvalue))
        (bind _out_row_2 (Utilities|WeaponData _output_get))
        (bind _returnvalue_2 (Transformation|AttachComponentToComponent (Variables|/Script/Engine.Actor|GetRootComponent _output_get) (Variables|Default|GetPlayerMesh) (Utilities|Struct|BreakWeaponProperties _out_row_2) "SnapToTarget" "SnapToTarget" "SnapToTarget" true))
        (return _returnvalue_2)
        (else
          (return (LocalVariables|GetLFound?)))))))