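; Destroyable is an actor Blueprint that takes damage and explodes when its Life runs out.
; Any damage reduces Life, and at zero or below it plays a grenade launcher explosion sound and particle effect at its location, then destroys itself.
; On BeginPlay it caches a controller obtained from the first player controller, printing an error if invalid, though nothing else here uses it.
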(event EventBeginPlay
  ;[1 1 1] Begin Play
  (bind _controller (Class|BPIPlayerController|GetController(Message) (Game|GetPlayerController 0)))
  (Utilities|IsValid _controller
    (:Is%20Valid
      (Variables|Default|SetController _controller))
    (:Is%20Not%20Valid
      (Development|PrintString "Destroyable : PC NOT VALID" true true "(R=0.640625,G=0.000000,B=0.016382,A=1.000000)" 5.0))))

(event Collision|EventActorBeginOverlap
  (params (OtherActor :type Actor%20Object%20Reference)))

(event EventTick
  (params (DeltaSeconds :type Float%20%28single-precision%29)))

(event Game|Damage|EventAnyDamage
  (params (Damage :type Float%20%28single-precision%29) (DamageType :type Damage%20Type%20Object%20Reference) (InstigatedBy :type Controller%20Object%20Reference) (DamageCauser :type Actor%20Object%20Reference))
  (bind _returnvalue (Transformation|GetActorLocation))
  ;[1 1 1] Damaged
  (Variables|Default|SetLife (- (Variables|Default|GetLife) Damage))
  (if (<= (Variables|Default|GetLife) 0.0)
    (Audio|PlaySoundatLocation "/Game/Marketplace/PrototypeWeap/Sound/GrenadeLauncher/GL_Explosion_Cue.GL_Explosion_Cue" _returnvalue "0, 0, 0" 2.0 1.0 0.0 0 0 0 0)
    (Effects|SpawnEmitteratLocation "/Game/Marketplace/PrototypeWeap/FX/P_GrenadeLauncher_Explosion_01.P_GrenadeLauncher_Explosion_01" _returnvalue)
    (Actor|DestroyActor)))

(fn ConstructionScript)