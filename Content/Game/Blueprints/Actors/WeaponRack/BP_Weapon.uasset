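; BP_Weapon is a weapon actor, filed under WeaponRack, that takes its appearance from gun data.
; Its construction script looks up the GunData ID row in its data table, when that table is valid, and applies the row's GunMesh to the WeaponMesh skeletal mesh component.
; GetWeapon returns the actor itself, and the event graph has no active logic.
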(event EventBeginPlay)

(event Collision|EventActorBeginOverlap
  (params (OtherActor :type Actor%20Object%20Reference)))

(event EventTick
  (params (DeltaSeconds :type Float%20%28single-precision%29)))

(fn ConstructionScript
  (bind _gundata (Variables|Default|GetGunData))
  (bind _id (Utilities|Struct|BreakWeaponProperties _gundata))
  (bind (_datatable _rowname) (Utilities|Struct|BreakDataTableRowHandle _id))
  (Utilities|IsValid _datatable
    (:Is%20Valid
      (bind _returnvalue (Utilities|GetDataTableRow _datatable _rowname)
        (:then
          (Components|SkeletalMesh|SetSkeletalMeshAsset (Variables|Default|GetWeaponMesh) (.GunMesh (Utilities|Struct|BreakWeaponProperties _returnvalue))))))))

(fn GetWeapon
  (return self))