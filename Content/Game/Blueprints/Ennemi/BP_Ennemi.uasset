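; BP_Ennemi is an enemy that hurts the third-person player and explodes with sound and particles when its life runs out.
; Overlapping its DamageHitBox starts a looping timer that applies damage at HitPerSecond, with a negative start delay for an immediate first hit; nothing here clears it.
; The construction script tints two mesh material slots with BodyColor through dynamic material instances.
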(event OnComponentBeginOverlap(DamageHitBox)
  (params (OverlappedComponent :type Primitive%20Component%20Object%20Reference) (OtherActor :type Actor%20Object%20Reference) (OtherComp :type Primitive%20Component%20Object%20Reference) (OtherBodyIndex :type Integer) (bFromSweep :type Boolean) (SweepResult :type Hit%20Result%20Structure%20%28by%20ref%29))
  (bind _hitpersecond (Variables|Default|GetHitPerSecond))
  (bind _returnvalue (/ 1.0 _hitpersecond))
  ;[1 1 1] Damage Player
  (bind _asbp_third_person_character (Utilities|Casting|CastToBP_ThirdPersonCharacter OtherActor))
  (Variables|Default|SetPlayer _asbp_third_person_character)
  (Utilities|Time|SetTimerbyFunctionName 0 "ApplyDamage" _returnvalue true (* _returnvalue -1.0)))

(event Collision|EventActorBeginOverlap
  (params (OtherActor :type Actor%20Object%20Reference)))

(event EventTick
  (params (DeltaSeconds :type Float%20%28single-precision%29)))

(event Game|Damage|EventAnyDamage
  (params (Damage :type Float%20%28single-precision%29) (DamageType :type Damage%20Type%20Object%20Reference) (InstigatedBy :type Controller%20Object%20Reference) (DamageCauser :type Actor%20Object%20Reference))
  (bind _returnvalue (Transformation|GetActorLocation))
  ;[1 1 1] Damaged
  (Variables|Default|SetLife (- (Variables|Default|GetLife) Damage))
  (if (<= (Variables|Default|GetLife) 0.0)
    (Audio|PlaySoundatLocation "/Game/Marketplace/PrototypeWeap/Sound/GrenadeLauncher/GL_Explosion_Cue.GL_Explosion_Cue" _returnvalue "0, 0, 0" 1.0 1.0 0.0 0 0 0 0)
    (Effects|SpawnEmitteratLocation "/Game/Marketplace/PrototypeWeap/FX/P_GrenadeLauncher_Explosion_01.P_GrenadeLauncher_Explosion_01" _returnvalue "0, 0, 0" "0.500000,0.500000,0.500000")
    (Actor|DestroyActor)))

(fn ConstructionScript
  (CallFunction|ChangeBodyCollor))

(fn ChangeBodyCollor
  (bind _mesh (Variables|Character|GetMesh))
  (bind _bodycolor (Variables|Default|GetBodyColor))
  ;[1 1 1] Change body color
  (bind _returnvalue (Rendering|Material|CreateDynamicMaterialInstance _mesh 0 0 "None" :!class /Script/Engine.PrimitiveComponent))
  (Rendering|Material|SetVectorParameterValue _returnvalue "Tint" _bodycolor :!class /Script/Engine.MaterialInstanceDynamic)
  (bind _returnvalue_2 (Rendering|Material|CreateDynamicMaterialInstance _mesh 1 0 "None" :!class /Script/Engine.PrimitiveComponent))
  (Rendering|Material|SetVectorParameterValue _returnvalue_2 "Tint" _bodycolor :!class /Script/Engine.MaterialInstanceDynamic)
  (return))

(fn ApplyDamage
  (Game|Damage|ApplyDamage (Variables|Default|GetPlayer) (Variables|Default|GetDamageAmmount) 0 self))