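; Stationary shooting enemy that turns to face the player character when Pawn Sensing spots it and fires projectiles.
; A flag adds a delay before its first reaction, and a second flag with a short cooldown limits fire rate.
; Incoming damage drains Life until it explodes with sound and particles and is destroyed.
; The construction script tints two mesh material slots with BodyColor through dynamic material instances.
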(event OnSeePawn(PawnSensing)
  (params (Pawn :type Pawn%20Object%20Reference))
  (bind _asbp_third_person_character (Utilities|Casting|CastToBP_ThirdPersonCharacter Pawn))
  (if (Variables|Default|GetwaitTime)
    (Utilities|FlowControl|Delay 3.0)
    (Variables|Default|SetwaitTime false))
  (Transformation|SetActorRotation (Math|Rotator|FindRelativeLookatRotation (Math|Conversions|ToTransform(Vector) (Transformation|GetActorLocation)) (Transformation|GetActorLocation _asbp_third_person_character)))
  (if (Variables|Default|GetCan%20Shoot)
    (Game|SpawnActorfromClass "/Game/Game/Blueprints/Actors/WeaponRack/BP_EnemyProjectile.BP_EnemyProjectile_C" (Transformation|GetWorldTransform (Variables|Default|GetProjectileLocaion)) "Undefined" 0 0)
    (Variables|Default|SetCan%20Shoot false)
    (Utilities|FlowControl|Delay 0.5)
    (Variables|Default|SetCan%20Shoot true)))

(event Game|Damage|EventAnyDamage
  (params (Damage :type Float%20%28single-precision%29) (DamageType :type Damage%20Type%20Object%20Reference) (InstigatedBy :type Controller%20Object%20Reference) (DamageCauser :type Actor%20Object%20Reference))
  (bind _returnvalue (Transformation|GetActorLocation))
  ;[1 1 1] Damaged
  (Variables|Default|SetLife (- (Variables|Default|GetLife) Damage))
  (if (<= (Variables|Default|GetLife) 0.0)
    (Audio|PlaySoundatLocation "/Game/Marketplace/PrototypeWeap/Sound/GrenadeLauncher/GL_Explosion_Cue.GL_Explosion_Cue" _returnvalue "0, 0, 0" 1.0 1.0 0.0 0 0 0 0)
    (Effects|SpawnEmitteratLocation "/Game/Marketplace/PrototypeWeap/FX/P_GrenadeLauncher_Explosion_01.P_GrenadeLauncher_Explosion_01" _returnvalue "0, 0, 0" "0.500000,0.500000,0.500000")
    (Actor|DestroyActor)))

(fn ConstructionScript
  (CallFunction|ChangeBodyCollor))

(fn ApplyDamage
  (Game|Damage|ApplyDamage (Variables|Default|GetPlayer) 0.0 0 self))

(fn ChangeBodyCollor
  (bind _bodycolor (Variables|Default|GetBodyColor))
  (bind _mesh (Variables|Character|GetMesh))
  ;[1 1 1] Change body color
  (bind _returnvalue (Rendering|Material|CreateDynamicMaterialInstance _mesh 0 0 "None" :!class /Script/Engine.PrimitiveComponent))
  (Rendering|Material|SetVectorParameterValue _returnvalue "Tint" _bodycolor :!class /Script/Engine.MaterialInstanceDynamic)
  (bind _returnvalue_2 (Rendering|Material|CreateDynamicMaterialInstance _mesh 1 0 "None" :!class /Script/Engine.PrimitiveComponent))
  (Rendering|Material|SetVectorParameterValue _returnvalue_2 "Tint" _bodycolor :!class /Script/Engine.MaterialInstanceDynamic)
  (return))