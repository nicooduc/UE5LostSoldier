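; Stationary shooter enemy that turns toward and attacks the third-person player character when PawnSensing sees it.
; Each shot spawns an actor at the projectile arrow and applies damage directly to the player, gated by a short CanShoot cooldown.
; Incoming damage drains Life until it explodes and is destroyed.
; The construction script tints the body materials; timer-based repeat damage exists but is unwired.
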(event OnSeePawn(PawnSensing)
  (params (Pawn :type Pawn%20Object%20Reference))
  (Development|PrintString "SEE")
  (bind _asbp_third_person_character (Utilities|Casting|CastToBP_ThirdPersonCharacter Pawn))
  (Transformation|SetActorRotation (Math|Rotator|FindRelativeLookatRotation (Math|Conversions|ToTransform(Vector) (Transformation|GetActorLocation)) (Transformation|GetActorLocation _asbp_third_person_character)))
  (if (Variables|Default|GetCanShoot)
    (Game|SpawnActorfromClass "/Game/Game/Blueprints/Actors/WeaponRack/BP_Projectile.BP_Projectile_C" (Transformation|GetWorldTransform (Variables|Default|GetSpawnArrowProjectile)) "Undefined" 0 0)
    (Game|Damage|ApplyDamage _asbp_third_person_character 1.0 0 0)
    (Variables|Default|SetCanShoot false)
    (Utilities|FlowControl|Delay 0.5)
    (Variables|Default|SetCanShoot true)))

(event Collision|EventActorBeginOverlap
  (params (OtherActor :type Actor%20Object%20Reference)))

(event EventTick
  (params (DeltaSeconds :type Float%20%28single-precision%29)))

(event Game|Damage|EventAnyDamage
  (params (Damage :type Float%20%28single-precision%29) (DamageType :type Damage%20Type%20Object%20Reference) (InstigatedBy :type Controller%20Object%20Reference) (DamageCauser :type Actor%20Object%20Reference))
  (bind _returnvalue (Transformation|GetActorLocation))
  ;[1 1 1] Damaged
  (Variables|Default|SetLife (- (Variables|Default|GetLife) Damage))
  (if (<= (Variables|Default|GetLife) 0.0)
    (Audio|PlaySoundatLocation "/Game/Marketplace/PrototypeWeap/Sound/GrenadeLauncher/GL_Explosion_Cue.GL_Explosion_Cue" _returnvalue "0, 0, 0" 2.0 1.0 0.0 0 0 0 0)
    (Effects|SpawnEmitteratLocation "/Game/Marketplace/PrototypeWeap/FX/P_GrenadeLauncher_Explosion_01.P_GrenadeLauncher_Explosion_01" _returnvalue)
    (Actor|DestroyActor)))

(fn ConstructionScript
  (CallFunction|ChangeBodyCollor))

(fn ChangeBodyCollor
  (bind _mesh (Variables|Character|GetMesh))
  (bind _bodycolor (Variables|Default|GetBodyColor))
  ;[1 1 1] Change body color
  (bind _returnvalue (Rendering|Material|CreateDynamicMaterialInstance _mesh 0 0 "None" :!class /Script/Engine.PrimitiveComponent))
  (Rendering|Material|SetVectorParameterValue _returnvalue "Tint" _bodycolor :!class /Script/Engine.MaterialInstanceDynamic)
  (bind _returnvalue_2 (Rendering|Material|CreateDynamicMaterialInstance _mesh 1 0 "None" :!class /Script/Engine.PrimitiveComponent))
  (Rendering|Material|SetVectorParameterValue _returnvalue_2 "Tint" _bodycolor :!class /Script/Engine.MaterialInstanceDynamic)
  (return))

(fn ApplyDamage
  (Game|Damage|ApplyDamage (Variables|Default|GetPlayer) (Variables|Default|GetDamageAmmount) 0 self))